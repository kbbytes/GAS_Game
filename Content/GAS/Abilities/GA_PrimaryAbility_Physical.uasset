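; GA_PrimaryAbility_Physical is a gameplay ability that fires a damage-carrying BP_Projectile from the third-person character.
; On activation it commits, builds a GE_Damage spec with a SetByCaller magnitude and a damage-type asset tag, and passes it to the projectile.
; The projectile spawns along the follow camera's forward vector, offset by the boom's arm length, then the ability ends immediately.
; An input-release debug print is left unconnected.
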(event `self.K2_ActivateAbility`
  (bind _returnvalue (`self.GetAvatarActorFromActorInfo`))
  (`self.K2_CommitAbility`)
  (bind _asbp_third_person_character (cast `/Game/PlayerCharacter/BP_ThirdPersonCharacter` _returnvalue))
  (bind _returnvalue_2 (`AbilitySystemBlueprintLibrary.GetAbilitySystemComponent` _asbp_third_person_character))
  (bind _returnvalue_3 (`AbilitySystemBlueprintLibrary.AssignTagSetByCallerMagnitude` (`AbilitySystemComponent.MakeOutgoingSpec` _returnvalue_2 "/Game/GAS/Effects/GE_Damage.GE_Damage_C" 0.0 (`AbilitySystemComponent.MakeEffectContext` _returnvalue_2)) (struct :`TagName` "Damage.SetByCaller") (`self.Damage`)))
  (`AbilitySystemBlueprintLibrary.AddAssetTag` _returnvalue_3 (`self.DamageTypeTag`))
  (bind _followcamera (`GAS_GameCharacter.FollowCamera` _asbp_third_person_character))
  (bind _returnvalue_4 (`SceneComponent.K2_GetComponentRotation` _followcamera))
  (`|SpawnActorFromClass` "/Game/Blueprints/BP_Projectile.BP_Projectile_C" (`KismetMathLibrary.MakeTransform` (+ (`SceneComponent.K2_GetComponentLocation` _followcamera) (* (`KismetMathLibrary.GetForwardVector` _returnvalue_4) (`SpringArmComponent.TargetArmLength` (`GAS_GameCharacter.CameraBoom` _asbp_third_person_character)))) _returnvalue_4 (0.4 0.4 0.4)) "Undefined" "MultiplyWithRoot" _returnvalue _returnvalue_3 null)
  (`self.K2_EndAbility`))